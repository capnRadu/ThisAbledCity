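; BP_DoorMaddie is an interactable door that transports the player to the Maddie level.
; Its sphere overlap shows a single P_interact prompt for BP_PlayerWheelchair and removes it when the player leaves.
; Interact plays a click sound and a WB_Fade animation, waits briefly, sets the GameInstance's spawn tag to MaddieRoom, then opens the level.
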(event OnComponentBeginOverlap(Sphere)
  (params (OverlappedComponent :type Primitive%20Component%20Object%20Reference) (OtherActor :type Actor%20Object%20Reference) (OtherComp :type Primitive%20Component%20Object%20Reference) (OtherBodyIndex :type Integer) (bFromSweep :type Boolean) (SweepResult :type Hit%20Result%20Structure%20%28by%20ref%29))
  ;[0.15 0.15 0.15 0.5] Press E to interact prompt pop up
  ;;[0.15 0.15 0.15 0.5] Check if the other actor is not self (most likely not, but better be sure)
  (if (!= OtherActor self)
    ;;[0.15 0.15 0.15 0.5] Check if the other actor is the player and also if the interact prompt doesn't exist (this prevents multiple prompts appearing if the begin overlap event is triggered more than once)
    (Utilities|Casting|CastToBP_PlayerWheelchair OtherActor)
    (Utilities|IsValid (Variables|Default|GetInteractPrompt)
      (:Is%20Not%20Valid
        ;;[0.15 0.15 0.15 0.5] Create widget, set variable, add to screen
        (bind _returnvalue (UserInterface|CreateWidget "/Game/Maps/Leisa/P_interact.P_interact_C"))
        (bind _output_get (Variables|Default|SetInteractPrompt _returnvalue))
        (UserInterface|Viewport|AddtoViewport _output_get 0)))))

(event OnComponentEndOverlap(Sphere)
  (params (OverlappedComponent :type Primitive%20Component%20Object%20Reference) (OtherActor :type Actor%20Object%20Reference) (OtherComp :type Primitive%20Component%20Object%20Reference) (OtherBodyIndex :type Integer))
  ;[0.15 0.15 0.15 0.5] Press E to interact prompt pop up
  ;;[0.15 0.15 0.15 0.5] Same as above
  (if (!= OtherActor self)
    ;;[0.15 0.15 0.15 0.5] First check if the variable exists (meaning the widget is on screen), and only then proceed to check if the other actor is the player
    (Utilities|IsValid (Variables|Default|GetInteractPrompt)
      (:Is%20Valid
        (Utilities|Casting|CastToBP_PlayerWheelchair OtherActor)
        ;;[0.15 0.15 0.15 0.5] Remove widget and clear variable
        (Widget|RemovefromParent (Variables|Default|GetInteractPrompt))
        (Variables|Default|SetInteractPrompt 0)))))

(event EventInteract
  (params (PlayerRef :type BP%20Player%20Wheelchair%20Object%20Reference))
  ;[0.15 0.15 0.15 0.5] Interact, play sound and open scene
  (bind _asbp_game_instance (Utilities|Casting|CastToBP_GameInstance (Game|GetGameInstance)))
  (Audio|PlaySound2D "/Game/Sounds/mouse-click-290204.mouse-click-290204" 1.0 1.0 0.0 0 0)
  (bind _returnvalue (UserInterface|CreateWidget "/Game/Maps/Leisa/WB_Fade.WB_Fade_C"))
  (UserInterface|Viewport|AddtoViewport _returnvalue 0)
  (Default|FadeAnim _returnvalue)
  (Utilities|FlowControl|Delay 0.5)
  (Variables|/Game/Blueprints/Radu/GameInstances/BP_GameInstance.BP_GameInstance_C|SetChosenPlayerStartTag _asbp_game_instance "MaddieRoom")
  (Game|OpenLevel(byName) "Maddie"))

(fn ConstructionScript)