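; Blueprint for inaccessible stairs on the Leisa map that can be reconstructed into an accessible version, extending a parent class that defines the mesh-switch events.
; Switching to the reconstruction mesh runs the parent logic, shows the warning tape and calls Activate on the sparkles without reset.
; Transforming to accessible hides the cube and tape, disables the cube's collision, reveals the reconstruction mesh with full collision and activates the sparkles.
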(event EventSwitchtoReconstructionMesh
  (|CallParentFunction)
  (Rendering|SetVisibility (Variables|Default|GetWarningTape) true false)
  (Components|Activation|Activate (Variables|Default|GetSparkles) false))

(event EventTransformMeshtoAccessible
  (bind _cube (Variables|Default|GetCube))
  (bind _reconstruction (Variables|Default|GetReconstruction))
  (|CallParentFunction)
  (Rendering|SetVisibility _cube false false)
  (Collision|SetCollisionEnabled _cube "NoCollision")
  (Rendering|SetVisibility (Variables|Default|GetWarningTape) false false)
  (Rendering|SetVisibility _reconstruction true false)
  (Collision|SetCollisionEnabled _reconstruction "QueryAndPhysics")
  (Components|Activation|Activate (Variables|Default|GetSparkles) false))

(fn ConstructionScript
  (|CallParentFunction))