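; BP_SemLobby is an interactable level transition that sends the player to DaniMap at the "SemLobby" player start.
; On Interact it plays a click sound, runs a WB_Fade animation, waits briefly, stores the start tag in BP_GameInstance and opens the level.
; The sphere overlap events are empty; their logic for showing and removing a P_interact prompt for BP_PlayerWheelchair is disconnected and never runs.
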(event OnComponentBeginOverlap(Sphere)
  (params (OverlappedComponent :type Primitive%20Component%20Object%20Reference) (OtherActor :type Actor%20Object%20Reference) (OtherComp :type Primitive%20Component%20Object%20Reference) (OtherBodyIndex :type Integer) (bFromSweep :type Boolean) (SweepResult :type Hit%20Result%20Structure%20%28by%20ref%29))
  ;[0.15 0.15 0.15 0.5] Press E to interact prompt pop up
)

(event OnComponentEndOverlap(Sphere)
  (params (OverlappedComponent :type Primitive%20Component%20Object%20Reference) (OtherActor :type Actor%20Object%20Reference) (OtherComp :type Primitive%20Component%20Object%20Reference) (OtherBodyIndex :type Integer))
  ;[0.15 0.15 0.15 0.5] Press E to interact prompt pop up
)

(event EventInteract
  (params (PlayerRef :type BP%20Player%20Wheelchair%20Object%20Reference))
  ;[0.15 0.15 0.15 0.5] Interact, play sound and open scene
  (bind _asbp_game_instance (Utilities|Casting|CastToBP_GameInstance (Game|GetGameInstance)))
  (Audio|PlaySound2D "/Game/Sounds/mouse-click-290204.mouse-click-290204" 1.0 1.0 0.0 0 0)
  (bind _returnvalue (UserInterface|CreateWidget "/Game/Maps/Leisa/WB_Fade.WB_Fade_C"))
  (UserInterface|Viewport|AddtoViewport _returnvalue 0)
  (Default|FadeAnim _returnvalue)
  (Utilities|FlowControl|Delay 0.5)
  (Variables|/Game/Blueprints/Radu/GameInstances/BP_GameInstance.BP_GameInstance_C|SetChosenPlayerStartTag _asbp_game_instance "SemLobby")
  (Game|OpenLevel(byName) "DaniMap"))

(fn ConstructionScript)