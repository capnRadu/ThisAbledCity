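; Dialogue component that runs data-table-driven conversations through an on-screen dialogue widget.
; Each Interact shows the current row's text and stores the next row, table and end flag, removing the widget on the interaction after an end row.
; Option buttons are added only when the widget is first created from an open-ended row.
; OptionSelected jumps the conversation to a supplied row and table.
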(event Custom|Option%20Selected
  (params (RowName :type Name) (DataTable :type Data%20Table%20Object%20Reference))
  (bind _returnvalue (Utilities|GetDataTableRow DataTable RowName)
    (:then
      (Default|UpdateDialogue (Variables|Default|GetDialogueWidget) (.Dialogue (Utilities|Struct|BreakBP_Dialogue_Structure _returnvalue)))
      (Variables|Default|SetRow%20Name%20Var (.Row (Utilities|Struct|BreakBP_Dialogue_Structure _returnvalue)))
      (Variables|Default|SetData%20Table%20Var (.DataTable (Utilities|Struct|BreakBP_Dialogue_Structure _returnvalue)))
      (Variables|Default|SetEndDialogue (.EndDialogue (Utilities|Struct|BreakBP_Dialogue_Structure _returnvalue))))
    (:RowNotFound
      (Development|PrintString "Options NOT WORKING"))))

(event EventInteract
  (params (PlayerRef :type BP%20Player%20Wheelchair%20Object%20Reference))
  (if (Variables|Default|GetEndDialogue)
    (Widget|RemovefromParent (Variables|Default|GetDialogueWidget))
    (Variables|Default|SetEndDialogue false)
    (Variables|Default|SetDialogueWidget 0)
    (else
      (Utilities|IsValid (Variables|Default|GetDialogueWidget)
        (:Is%20Valid
          (bind _returnvalue (Utilities|GetDataTableRow (Variables|Default|GetData%20Table%20Var) (Variables|Default|GetRow%20Name%20Var))
            (:then
              (Default|UpdateDialogue (Variables|Default|GetDialogueWidget) (.Dialogue (Utilities|Struct|BreakBP_Dialogue_Structure _returnvalue)))
              (Variables|Default|SetRow%20Name%20Var (.Row (Utilities|Struct|BreakBP_Dialogue_Structure _returnvalue)))
              (Variables|Default|SetData%20Table%20Var (.DataTable (Utilities|Struct|BreakBP_Dialogue_Structure _returnvalue)))
              (Variables|Default|SetEndDialogue (.EndDialogue (Utilities|Struct|BreakBP_Dialogue_Structure _returnvalue))))
            (:RowNotFound
              (Development|PrintString "OWO" :!label _label))))
        (:Is%20Not%20Valid
          (bind _returnvalue_2 (Utilities|GetDataTableRow (Variables|Default|GetData%20Table%20Var) (Variables|Default|GetRow%20Name%20Var))
            (:then
              (bind _returnvalue_3 (UserInterface|CreateWidget "/Game/Blueprints/Max/DialogueSystem/WBP_Dialogue.WBP_Dialogue_C" 0 (Utilities|Text|ToText(Name) (Variables|Default|GetName)) (.Dialogue (Utilities|Struct|BreakBP_Dialogue_Structure _returnvalue_2))))
              (bind _output_get (Variables|Default|SetDialogueWidget _returnvalue_3))
              (UserInterface|Viewport|AddtoViewport _output_get 0)
              (Variables|Default|SetRow%20Name%20Var (.Row (Utilities|Struct|BreakBP_Dialogue_Structure _returnvalue_2)))
              (Variables|Default|SetData%20Table%20Var (.DataTable (Utilities|Struct|BreakBP_Dialogue_Structure _returnvalue_2)))
              (Variables|Default|SetEndDialogue (.EndDialogue (Utilities|Struct|BreakBP_Dialogue_Structure _returnvalue_2)))
              (if (.OpenEndedDialogue? (Utilities|Struct|BreakBP_Dialogue_Structure _returnvalue_2))
                (for _array_element (.OpenEndedDialogueOptions (Utilities|Struct|BreakBP_Dialogue_Structure _returnvalue_2))
                  (bind _returnvalue_4 (UserInterface|CreateWidget "/Game/Blueprints/Max/DialogueSystem/WBP_DialogueOptions.WBP_DialogueOptions_C" 0 (Utilities|Text|ToText(Name) (.OptionName (Utilities|Struct|BreakBP_OptionsDialogue_structure _array_element)))))
                  (Widget|Panel|AddChild (Variables|/Game/Blueprints/Max/DialogueSystem/WBP_Dialogue.WBP_Dialogue_C|GetVar_DialogueScrollBox (Variables|Default|GetDialogueWidget)) _returnvalue_4))))
            (:RowNotFound
              (goto _label))))))))