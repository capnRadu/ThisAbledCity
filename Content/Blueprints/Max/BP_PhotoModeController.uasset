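; BP_PhotoModeController is the possessed free-camera pawn for photo mode.
; Look inputs steer the control rotation, with both raw and CameraMovementSpeed-scaled handlers, and movement follows that rotation plus world-up for vertical travel.
; Forward and right inputs also print their axis values to screen.
; Pressing CameraMode makes PlayerController re-possess the stored Player, then destroys this actor.
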(event Input|ActionEvents|InputActionCameraMode
  (params (Key :type Key%20Structure :default "None"))
  (:Pressed
    (Pawn|Possess (Variables|Default|GetPlayerController) (Variables|Default|GetPlayer))
    (Actor|DestroyActor)))

(event Input|AxisEvents|InputAxisMoveForward
  (params (AxisValue :type Float%20%28single-precision%29))
  (Development|PrintString (Utilities|String|ToString(Float) AxisValue) true true "(R=0.000000,G=0.660000,B=1.000000,A=1.000000)" 5.0)
  (Pawn|Input|AddMovementInput (Math|Vector|GetForwardVector (Pawn|GetControlRotation :!class /Script/Engine.Pawn)) AxisValue false))

(event Input|AxisEvents|InputAxisMoveRight
  (params (AxisValue :type Float%20%28single-precision%29))
  (Development|PrintString (Utilities|String|ToString(Float) AxisValue) true true "(R=0.000000,G=0.660000,B=1.000000,A=1.000000)" 5.0)
  (Pawn|Input|AddMovementInput (Math|Vector|GetRightVector (Pawn|GetControlRotation :!class /Script/Engine.Pawn)) AxisValue false))

(event Input|AxisEvents|InputAxisMoveUp
  (params (AxisValue :type Float%20%28single-precision%29))
  (Pawn|Input|AddMovementInput "0.000000,0.000000,1.000000" AxisValue false))

(event Input|AxisEvents|InputAxisLookUp
  (params (AxisValue :type Float%20%28single-precision%29))
  (Pawn|Input|AddControllerPitchInput AxisValue))

(event Input|AxisEvents|InputAxisTurn
  (params (AxisValue :type Float%20%28single-precision%29))
  (Pawn|Input|AddControllerYawInput AxisValue))

(event Input|AxisEvents|InputAxisLookUpRate
  (params (AxisValue :type Float%20%28single-precision%29))
  (Pawn|Input|AddControllerPitchInput (* AxisValue (Variables|Default|GetCamera%20Movement%20Speed) (Utilities|Time|GetWorldDeltaSeconds))))

(event Input|AxisEvents|InputAxisTurn
  (params (AxisValue :type Float%20%28single-precision%29))
  (Pawn|Input|AddControllerYawInput (* AxisValue (Variables|Default|GetCamera%20Movement%20Speed) (Utilities|Time|GetWorldDeltaSeconds))))

(fn ConstructionScript)