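; GM_Base is a game mode Blueprint that decides which PlayerStart a player spawns at.
; Its ChoosePlayerStart override reads ChosenPlayerStartTag from BP_GameInstance and returns the first PlayerStart carrying that tag, without checking that one exists.
; When the tag is None, it uses the first start tagged LobbyDoor, falling back to the parent implementation if none is found.
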(event EventBeginPlay)

(event EventTick
  (params (DeltaSeconds :type Float%20%28single-precision%29)))

(fn ConstructionScript)

(fn ChoosePlayerStart
  (params (Player :type Controller%20Object%20Reference))
  (bind _asbp_game_instance (Utilities|Casting|CastToBP_GameInstance (Game|GetGameInstance)))
  (if (== (Variables|/Game/Blueprints/Radu/GameInstances/BP_GameInstance.BP_GameInstance_C|GetChosenPlayerStartTag _asbp_game_instance) "")
    (bind _outactors (Actor|GetAllActorsOfClasswithTag "/Script/Engine.PlayerStart" "LobbyDoor"))
    (if (!= (Utilities|Array|Length _outactors) 0)
      (return (Utilities|Array|Get(acopy) _outactors))
      (else
        (bind _returnvalue (|CallParentFunction Player))
        (return _returnvalue)))
    (else
      (bind _outactors_2 (Actor|GetAllActorsOfClasswithTag "/Script/Engine.PlayerStart" (Variables|/Game/Blueprints/Radu/GameInstances/BP_GameInstance.BP_GameInstance_C|GetChosenPlayerStartTag _asbp_game_instance)))
      (return (Utilities|Array|Get(acopy) _outactors_2)))))