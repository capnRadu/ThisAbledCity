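; Player controller for the wheelchair pawn, mapping keyboard and gamepad Enhanced Input to driving, camera and menu actions.
; BeginPlay caches the pawn, adds both mapping contexts and registers contexts with user settings.
; Throttle, steering and brake feed the vehicle movement component, with flags making forward throttle and brake mutually exclusive.
; It also forwards camera switch, toggle and look inputs, and toggles a game-pausing menu and a non-pausing notebook widget.
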(event Custom|OpenNotebook
  (bind _self self)
  ;[0.15 0.15 0.15 0.5] General Inputs
  (bind _returnvalue (UserInterface|CreateWidget "/Game/Blueprints/Radu/Widgets/Notebook/WBP_Notebook.WBP_Notebook_C"))
  (bind _output_get (Variables|Default|SetNotebook _returnvalue))
  (UserInterface|Viewport|AddtoViewport _output_get 0)
  (Input|SetInputModeGameandUI _self _returnvalue "DoNotLock" true false)
  (Variables|/Script/Engine.PlayerController|SetbShowMouseCursor _self true)
  (Variables|Default|SetbEnableClickEvents _self true))

(event Custom|CloseNotebook
  (bind _self self)
  ;[0.15 0.15 0.15 0.5] General Inputs
  (Widget|RemovefromParent (Variables|Default|GetNotebook))
  (Variables|Default|SetNotebook 0)
  (Input|SetInputModeGameOnly _self false)
  (Variables|/Script/Engine.PlayerController|SetbShowMouseCursor _self false)
  (Variables|Default|SetbEnableClickEvents _self false))

(event Input|EnhancedActionEvents|EnhancedInputActionIA_PauseGamepad
  (params (ActionValue :type Boolean) (ElapsedSeconds :type Float%20%28double-precision%29) (TriggeredSeconds :type Float%20%28double-precision%29) (InputAction :type Input%20Action%20Object%20Reference :default "/Game/Input/Actions/PlayerWheelchair/Gamepad/IA_PauseGamepad.IA_PauseGamepad"))
  (bind _self self)
  (bind _self_2 self)
  ;[0.15 0.15 0.15 0.5] General Inputs
  (:Started
    (Utilities|IsValid (Variables|Default|GetPauseMenu)
      (:Is%20Valid
        (Widget|RemovefromParent (Variables|Default|GetPauseMenu))
        (Variables|Default|SetPauseMenu 0)
        (Input|SetInputModeGameOnly _self_2 false)
        (Variables|/Script/Engine.PlayerController|SetbShowMouseCursor _self_2 false)
        (Variables|Default|SetbEnableClickEvents _self_2 false)
        (Game|SetGamePaused false))
      (:Is%20Not%20Valid
        (bind _returnvalue (UserInterface|CreateWidget "/Game/Blueprints/Radu/Widgets/PauseMenuAndMappings/WBP_PauseMenu.WBP_PauseMenu_C" 0 self))
        (bind _output_get (Variables|Default|SetPauseMenu _returnvalue))
        (UserInterface|Viewport|AddtoViewport _output_get 0)
        (Input|SetInputModeGameandUI _self _returnvalue "DoNotLock" true false)
        (Variables|/Script/Engine.PlayerController|SetbShowMouseCursor _self true)
        (Variables|Default|SetbEnableClickEvents _self true)
        (Game|SetGamePaused true)))))

(event Input|EnhancedActionEvents|EnhancedInputActionIA_LookUpKeyboard
  (params (ActionValue :type Float%20%28double-precision%29) (ElapsedSeconds :type Float%20%28double-precision%29) (TriggeredSeconds :type Float%20%28double-precision%29) (InputAction :type Input%20Action%20Object%20Reference :default "/Game/Input/Actions/PlayerWheelchair/Keyboard/IA_LookUpKeyboard.IA_LookUpKeyboard"))
  ;[0.15 0.15 0.15 0.5] General Inputs
  (Pawn|Input|AddControllerPitchInput (Variables|Default|GetControlledPawn) (* ActionValue 8.0)))

(event Input|EnhancedActionEvents|EnhancedInputActionIA_ToggleCameraKeyboard
  (params (ActionValue :type Boolean) (ElapsedSeconds :type Float%20%28double-precision%29) (TriggeredSeconds :type Float%20%28double-precision%29) (InputAction :type Input%20Action%20Object%20Reference :default "/Game/Input/Actions/PlayerWheelchair/Keyboard/IA_ToggleCameraKeyboard.IA_ToggleCameraKeyboard"))
  ;[0.15 0.15 0.15 0.5] General Inputs
  (:Started
    (Default|OpenCamera (Variables|Default|GetBP_PlayerWheelchair))))

(event Input|EnhancedActionEvents|EnhancedInputActionIA_ThrottleUpGamepad
  (params (ActionValue :type Float%20%28double-precision%29) (ElapsedSeconds :type Float%20%28double-precision%29) (TriggeredSeconds :type Float%20%28double-precision%29) (InputAction :type Input%20Action%20Object%20Reference :default "/Game/Input/Actions/PlayerWheelchair/Gamepad/IA_ThrottleUpGamepad.IA_ThrottleUpGamepad"))
  ;[0.15 0.15 0.15 0.5] Throttle and Brake Inputs
  (:Triggered
    (if (not (Variables|Default|GetBrakePressed))
      (Variables|Default|SetThrottleUpPressed true)
      (Class|ChaosVehicleMovementComponent|SetThrottleInput (Variables|/Script/ChaosVehicles.WheeledVehiclePawn|GetVehicleMovementComponent (Variables|Default|GetBP_PlayerWheelchair)) ActionValue :!label _label)))
  (:Completed
    (Variables|Default|SetThrottleUpPressed false)
    (goto _label)))

(event Input|EnhancedActionEvents|EnhancedInputActionIA_ThrottleDownGamepad
  (params (ActionValue :type Float%20%28double-precision%29) (ElapsedSeconds :type Float%20%28double-precision%29) (TriggeredSeconds :type Float%20%28double-precision%29) (InputAction :type Input%20Action%20Object%20Reference :default "/Game/Input/Actions/PlayerWheelchair/Gamepad/IA_ThrottleDownGamepad.IA_ThrottleDownGamepad"))
  ;[0.15 0.15 0.15 0.5] Throttle and Brake Inputs
  (:Triggered
    (Class|ChaosVehicleMovementComponent|SetThrottleInput (Variables|/Script/ChaosVehicles.WheeledVehiclePawn|GetVehicleMovementComponent (Variables|Default|GetBP_PlayerWheelchair)) ActionValue :!label _label))
  (:Completed
    (goto _label)))

(event Input|EnhancedActionEvents|EnhancedInputActionIA_BrakeGamepad
  (params (ActionValue :type Float%20%28double-precision%29) (ElapsedSeconds :type Float%20%28double-precision%29) (TriggeredSeconds :type Float%20%28double-precision%29) (InputAction :type Input%20Action%20Object%20Reference :default "/Game/Input/Actions/PlayerWheelchair/Gamepad/IA_BrakeGamepad.IA_BrakeGamepad"))
  ;[0.15 0.15 0.15 0.5] Throttle and Brake Inputs
  (:Triggered
    (if (not (Variables|Default|GetThrottleUpPressed))
      (Variables|Default|SetBrakePressed true)
      (Class|ChaosVehicleMovementComponent|SetBrakeInput (Variables|/Script/ChaosVehicles.WheeledVehiclePawn|GetVehicleMovementComponent (Variables|Default|GetBP_PlayerWheelchair)) ActionValue :!label _label)))
  (:Completed
    (Variables|Default|SetBrakePressed false)
    (goto _label)))

(event Input|EnhancedActionEvents|EnhancedInputActionIA_SteeringLeftGamepad
  (params (ActionValue :type Float%20%28double-precision%29) (ElapsedSeconds :type Float%20%28double-precision%29) (TriggeredSeconds :type Float%20%28double-precision%29) (InputAction :type Input%20Action%20Object%20Reference :default "/Game/Input/Actions/PlayerWheelchair/Gamepad/IA_SteeringLeftGamepad.IA_SteeringLeftGamepad"))
  ;[0.15 0.15 0.15 0.5] Steering Inputs
  (:Triggered
    (Class|ChaosVehicleMovementComponent|SetSteeringInput (Variables|/Script/ChaosVehicles.WheeledVehiclePawn|GetVehicleMovementComponent (Variables|Default|GetBP_PlayerWheelchair)) ActionValue :!label _label))
  (:Completed
    (goto _label)))

(event Input|EnhancedActionEvents|EnhancedInputActionIA_SteeringRightGamepad
  (params (ActionValue :type Float%20%28double-precision%29) (ElapsedSeconds :type Float%20%28double-precision%29) (TriggeredSeconds :type Float%20%28double-precision%29) (InputAction :type Input%20Action%20Object%20Reference :default "/Game/Input/Actions/PlayerWheelchair/Gamepad/IA_SteeringRightGamepad.IA_SteeringRightGamepad"))
  ;[0.15 0.15 0.15 0.5] Steering Inputs
  (:Triggered
    (Class|ChaosVehicleMovementComponent|SetSteeringInput (Variables|/Script/ChaosVehicles.WheeledVehiclePawn|GetVehicleMovementComponent (Variables|Default|GetBP_PlayerWheelchair)) ActionValue :!label _label))
  (:Completed
    (goto _label)))

(event Input|EnhancedActionEvents|EnhancedInputActionIA_ToggleCameraGamepad
  (params (ActionValue :type Boolean) (ElapsedSeconds :type Float%20%28double-precision%29) (TriggeredSeconds :type Float%20%28double-precision%29) (InputAction :type Input%20Action%20Object%20Reference :default "/Game/Input/Actions/PlayerWheelchair/Gamepad/IA_ToggleCameraGamepad.IA_ToggleCameraGamepad"))
  ;[0.15 0.15 0.15 0.5] General Inputs
  (:Started
    (Default|OpenCamera (Variables|Default|GetBP_PlayerWheelchair))))

(event Input|EnhancedActionEvents|EnhancedInputActionIA_PauseKeyboard
  (params (ActionValue :type Boolean) (ElapsedSeconds :type Float%20%28double-precision%29) (TriggeredSeconds :type Float%20%28double-precision%29) (InputAction :type Input%20Action%20Object%20Reference :default "/Game/Input/Actions/PlayerWheelchair/Keyboard/IA_PauseKeyboard.IA_PauseKeyboard"))
  (bind _self self)
  (bind _self_2 self)
  ;[0.15 0.15 0.15 0.5] General Inputs
  (:Started
    (Utilities|IsValid (Variables|Default|GetPauseMenu)
      (:Is%20Valid
        (Widget|RemovefromParent (Variables|Default|GetPauseMenu))
        (Variables|Default|SetPauseMenu 0)
        (Input|SetInputModeGameOnly _self_2 false)
        (Variables|/Script/Engine.PlayerController|SetbShowMouseCursor _self_2 false)
        (Variables|Default|SetbEnableClickEvents _self_2 false)
        (Game|SetGamePaused false))
      (:Is%20Not%20Valid
        (bind _returnvalue (UserInterface|CreateWidget "/Game/Blueprints/Radu/Widgets/PauseMenuAndMappings/WBP_PauseMenu.WBP_PauseMenu_C" 0 self))
        (bind _output_get (Variables|Default|SetPauseMenu _returnvalue))
        (UserInterface|Viewport|AddtoViewport _output_get 0)
        (Input|SetInputModeGameandUI _self _returnvalue "DoNotLock" true false)
        (Variables|/Script/Engine.PlayerController|SetbShowMouseCursor _self true)
        (Variables|Default|SetbEnableClickEvents _self true)
        (Game|SetGamePaused true)))))

(event Input|EnhancedActionEvents|EnhancedInputActionIA_SwitchCamera
  (params (ActionValue :type Boolean) (ElapsedSeconds :type Float%20%28double-precision%29) (TriggeredSeconds :type Float%20%28double-precision%29) (InputAction :type Input%20Action%20Object%20Reference :default "/Game/Input/Actions/PlayerWheelchair/IA_SwitchCamera.IA_SwitchCamera"))
  ;[0.15 0.15 0.15 0.5] General Inputs
  (:Started
    (Default|ChangeCamera (Variables|Default|GetBP_PlayerWheelchair))))

(event Input|EnhancedActionEvents|EnhancedInputActionIA_TurnCameraKeyboard
  (params (ActionValue :type Float%20%28double-precision%29) (ElapsedSeconds :type Float%20%28double-precision%29) (TriggeredSeconds :type Float%20%28double-precision%29) (InputAction :type Input%20Action%20Object%20Reference :default "/Game/Input/Actions/PlayerWheelchair/Keyboard/IA_TurnCameraKeyboard.IA_TurnCameraKeyboard"))
  ;[0.15 0.15 0.15 0.5] General Inputs
  (Pawn|Input|AddControllerYawInput (Variables|Default|GetControlledPawn) (* ActionValue 8.0)))

(event Input|EnhancedActionEvents|EnhancedInputActionIA_ThrottleDownKeyboard
  (params (ActionValue :type Float%20%28double-precision%29) (ElapsedSeconds :type Float%20%28double-precision%29) (TriggeredSeconds :type Float%20%28double-precision%29) (InputAction :type Input%20Action%20Object%20Reference :default "/Game/Input/Actions/PlayerWheelchair/Keyboard/IA_ThrottleDownKeyboard.IA_ThrottleDownKeyboard"))
  ;[0.15 0.15 0.15 0.5] Throttle and Brake Inputs
  (:Triggered
    (Class|ChaosVehicleMovementComponent|SetThrottleInput (Variables|/Script/ChaosVehicles.WheeledVehiclePawn|GetVehicleMovementComponent (Variables|Default|GetBP_PlayerWheelchair)) ActionValue :!label _label))
  (:Completed
    (goto _label)))

(event Input|EnhancedActionEvents|EnhancedInputActionIA_SteeringLeftKeyboard
  (params (ActionValue :type Float%20%28double-precision%29) (ElapsedSeconds :type Float%20%28double-precision%29) (TriggeredSeconds :type Float%20%28double-precision%29) (InputAction :type Input%20Action%20Object%20Reference :default "/Game/Input/Actions/PlayerWheelchair/Keyboard/IA_SteeringLeftKeyboard.IA_SteeringLeftKeyboard"))
  ;[0.15 0.15 0.15 0.5] Steering Inputs
  (:Triggered
    (Class|ChaosVehicleMovementComponent|SetSteeringInput (Variables|/Script/ChaosVehicles.WheeledVehiclePawn|GetVehicleMovementComponent (Variables|Default|GetBP_PlayerWheelchair)) ActionValue :!label _label))
  (:Completed
    (goto _label)))

(event Input|EnhancedActionEvents|EnhancedInputActionIA_ThrottleUpKeyboard
  (params (ActionValue :type Float%20%28double-precision%29) (ElapsedSeconds :type Float%20%28double-precision%29) (TriggeredSeconds :type Float%20%28double-precision%29) (InputAction :type Input%20Action%20Object%20Reference :default "/Game/Input/Actions/PlayerWheelchair/Keyboard/IA_ThrottleUpKeyboard.IA_ThrottleUpKeyboard"))
  ;[0.15 0.15 0.15 0.5] Throttle and Brake Inputs
  (:Triggered
    (if (not (Variables|Default|GetBrakePressed))
      (Variables|Default|SetThrottleUpPressed true)
      (Class|ChaosVehicleMovementComponent|SetThrottleInput (Variables|/Script/ChaosVehicles.WheeledVehiclePawn|GetVehicleMovementComponent (Variables|Default|GetBP_PlayerWheelchair)) ActionValue :!label _label)))
  (:Completed
    (Variables|Default|SetThrottleUpPressed false)
    (goto _label)))

(event Input|EnhancedActionEvents|EnhancedInputActionIA_LookUpGamepad
  (params (ActionValue :type Float%20%28double-precision%29) (ElapsedSeconds :type Float%20%28double-precision%29) (TriggeredSeconds :type Float%20%28double-precision%29) (InputAction :type Input%20Action%20Object%20Reference :default "/Game/Input/Actions/PlayerWheelchair/Gamepad/IA_LookUpGamepad.IA_LookUpGamepad"))
  ;[0.15 0.15 0.15 0.5] General Inputs
  (Pawn|Input|AddControllerPitchInput (Variables|Default|GetControlledPawn) (* ActionValue 4e+01)))

(event Input|EnhancedActionEvents|EnhancedInputActionIA_TurnCameraGamepad
  (params (ActionValue :type Float%20%28double-precision%29) (ElapsedSeconds :type Float%20%28double-precision%29) (TriggeredSeconds :type Float%20%28double-precision%29) (InputAction :type Input%20Action%20Object%20Reference :default "/Game/Input/Actions/PlayerWheelchair/Gamepad/IA_TurnCameraGamepad.IA_TurnCameraGamepad"))
  ;[0.15 0.15 0.15 0.5] General Inputs
  (Pawn|Input|AddControllerYawInput (Variables|Default|GetControlledPawn) (* ActionValue 4e+01)))

(event Input|EnhancedActionEvents|EnhancedInputActionIA_SteeringRightKeyboard
  (params (ActionValue :type Float%20%28double-precision%29) (ElapsedSeconds :type Float%20%28double-precision%29) (TriggeredSeconds :type Float%20%28double-precision%29) (InputAction :type Input%20Action%20Object%20Reference :default "/Game/Input/Actions/PlayerWheelchair/Keyboard/IA_SteeringRightKeyboard.IA_SteeringRightKeyboard"))
  ;[0.15 0.15 0.15 0.5] Steering Inputs
  (:Triggered
    (Class|ChaosVehicleMovementComponent|SetSteeringInput (Variables|/Script/ChaosVehicles.WheeledVehiclePawn|GetVehicleMovementComponent (Variables|Default|GetBP_PlayerWheelchair)) ActionValue :!label _label))
  (:Completed
    (goto _label)))

(event Input|EnhancedActionEvents|EnhancedInputActionIA_NotebookKeyboard
  (params (ActionValue :type Boolean) (ElapsedSeconds :type Float%20%28double-precision%29) (TriggeredSeconds :type Float%20%28double-precision%29) (InputAction :type Input%20Action%20Object%20Reference :default "/Game/Input/Actions/PlayerWheelchair/Keyboard/IA_NotebookKeyboard.IA_NotebookKeyboard"))
  ;[0.15 0.15 0.15 0.5] General Inputs
  (:Started
    (Utilities|IsValid (Variables|Default|GetNotebook)
      (:Is%20Valid
        (CallFunction|CloseNotebook))
      (:Is%20Not%20Valid
        (CallFunction|OpenNotebook)))))

(event Input|EnhancedActionEvents|EnhancedInputActionIA_NotebookGamepad
  (params (ActionValue :type Boolean) (ElapsedSeconds :type Float%20%28double-precision%29) (TriggeredSeconds :type Float%20%28double-precision%29) (InputAction :type Input%20Action%20Object%20Reference :default "/Game/Input/Actions/PlayerWheelchair/Gamepad/IA_NotebookGamepad.IA_NotebookGamepad"))
  ;[0.15 0.15 0.15 0.5] General Inputs
  (:Started
    (Utilities|IsValid (Variables|Default|GetNotebook)
      (:Is%20Valid
        (CallFunction|CloseNotebook))
      (:Is%20Not%20Valid
        (CallFunction|OpenNotebook)))))

(event Input|EnhancedActionEvents|EnhancedInputActionIA_BrakeKeyboard
  (params (ActionValue :type Float%20%28double-precision%29) (ElapsedSeconds :type Float%20%28double-precision%29) (TriggeredSeconds :type Float%20%28double-precision%29) (InputAction :type Input%20Action%20Object%20Reference :default "/Game/Input/Actions/PlayerWheelchair/Keyboard/IA_BrakeKeyboard.IA_BrakeKeyboard"))
  ;[0.15 0.15 0.15 0.5] Throttle and Brake Inputs
  (:Triggered
    (if (not (Variables|Default|GetThrottleUpPressed))
      (Variables|Default|SetBrakePressed true)
      (Class|ChaosVehicleMovementComponent|SetBrakeInput (Variables|/Script/ChaosVehicles.WheeledVehiclePawn|GetVehicleMovementComponent (Variables|Default|GetBP_PlayerWheelchair)) ActionValue :!label _label)))
  (:Completed
    (Variables|Default|SetBrakePressed false)
    (goto _label)))

(event EventBeginPlay
  (bind _returnvalue (CallFunction|GetUserSettings))
  (bind _self self)
  (bind _returnvalue_2 (PlayerController|LocalPlayerSubsystems|GetEnhancedInputLocalPlayerSubsystem _self))
  (Utilities|FlowControl|Sequence
    (:then_0
      (bind _asbp_player_wheelchair (Utilities|Casting|CastToBP_PlayerWheelchair (Pawn|GetControlledPawn)))
      (bind _output_get (Variables|Default|SetBP_PlayerWheelchair _asbp_player_wheelchair))
      (Variables|Default|SetControlledPawn _output_get))
    (:then_1
      (Input|AddMappingContext _returnvalue_2 "/Game/Input/IMCs/WheelchairPlayer/IMC_PlayerWheelchairKeyboardControls.IMC_PlayerWheelchairKeyboardControls" 0 "(bIgnoreAllPressedKeysUntilRelease=True,bForceImmediately=False,bNotifyUserSettings=False)")
      (Input|AddMappingContext _returnvalue_2 "/Game/Input/IMCs/WheelchairPlayer/IMC_PlayerWheelchairGamepadControls.IMC_PlayerWheelchairGamepadControls" 0 "(bIgnoreAllPressedKeysUntilRelease=True,bForceImmediately=False,bNotifyUserSettings=False)")
      (for _array_element (CallFunction|GetAllInputMappingContexts)
        (if (not (Class|EnhancedInputUserSettings|IsMappingContextRegistered _returnvalue _array_element))
          (Class|EnhancedInputUserSettings|RegisterInputMappingContext _returnvalue _array_element))))))

(fn ConstructionScript)