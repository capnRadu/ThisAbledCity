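; Player wheelchair pawn with a switchable two-camera view, look limits relative to its facing, and level-specific quest starts on BeginPlay.
; OpenCamera stops movement and hands possession to a spawned photo-mode pawn, or repossesses the wheelchair and destroys that pawn.
; Overlap spheres track dialogue and interactable targets, which keyboard or gamepad interact input messages.
; Holding R grabs the traced component through a PhysicsHandle, whose target follows the camera each Tick.
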(event OnComponentBeginOverlap(DialogueSphere)
  (params (OverlappedComponent :type Primitive%20Component%20Object%20Reference) (OtherActor :type Actor%20Object%20Reference) (OtherComp :type Primitive%20Component%20Object%20Reference) (OtherBodyIndex :type Integer) (bFromSweep :type Boolean) (SweepResult :type Hit%20Result%20Structure%20%28by%20ref%29))
  (bind _returnvalue (Actor|GetComponentbyClass OtherActor "/Game/Blueprints/Max/DialogueSystem/BP_DialogueComponent.BP_DialogueComponent_C"))
  (Utilities|IsValid _returnvalue
    (:Is%20Valid
      (Variables|Default|SetTargetDialogueComponent _returnvalue))))

(event OnComponentEndOverlap(DialogueSphere)
  (params (OverlappedComponent :type Primitive%20Component%20Object%20Reference) (OtherActor :type Actor%20Object%20Reference) (OtherComp :type Primitive%20Component%20Object%20Reference) (OtherBodyIndex :type Integer))
  (Utilities|IsValid (Variables|Default|GetTargetDialogueComponent)
    (:Is%20Valid
      (Variables|Default|SetTargetDialogueComponent 0))))

(event OnComponentBeginOverlap(InteractSphere)
  (params (OverlappedComponent :type Primitive%20Component%20Object%20Reference) (OtherActor :type Actor%20Object%20Reference) (OtherComp :type Primitive%20Component%20Object%20Reference) (OtherBodyIndex :type Integer) (bFromSweep :type Boolean) (SweepResult :type Hit%20Result%20Structure%20%28by%20ref%29))
  (if (!= OtherActor self)
    (if (Utilities|DoesObjectImplementInterface OtherActor "/Game/Blueprints/Max/DialogueSystem/BP_Interact.BP_Interact_C")
      (Variables|Default|SetInteractActor OtherActor))))

(event OnComponentEndOverlap(InteractSphere)
  (params (OverlappedComponent :type Primitive%20Component%20Object%20Reference) (OtherActor :type Actor%20Object%20Reference) (OtherComp :type Primitive%20Component%20Object%20Reference) (OtherBodyIndex :type Integer))
  (Utilities|IsValid (Variables|Default|GetInteractActor)
    (:Is%20Valid
      (Variables|Default|SetInteractActor 0))))

(event Custom|ChangeCamera
  (bind _camera (Variables|Default|GetCamera))
  (bind _camera1 (Variables|Default|GetCamera1))
  (Components|Activation|SetActive _camera (not (Components|Activation|IsActive _camera)) false)
  (Components|Activation|SetActive _camera1 (not (Components|Activation|IsActive _camera1)) false))

(event Custom|OpenCamera
  (bind _playerwheelchaircontroller (Variables|Default|GetPlayerWheelchairController))
  (Utilities|IsValid (Variables|Default|GetPhotoModeController)
    (:Is%20Valid
      (Pawn|Possess (Variables|Default|GetPlayerWheelchairController) self)
      (Variables|/Game/Blueprints/Radu/Player/WheelchairController/BP_PlayerWheelchairController.BP_PlayerWheelchairController_C|SetControlledPawn _playerwheelchaircontroller (Variables|/Game/Blueprints/Radu/Player/WheelchairController/BP_PlayerWheelchairController.BP_PlayerWheelchairController_C|GetBP_PlayerWheelchair _playerwheelchaircontroller))
      (Actor|DestroyActor (Variables|Default|GetPhotoModeController)))
    (:Is%20Not%20Valid
      (Components|Movement|StopMovementImmediately (Variables|Default|GetVehicleMovementComponent))
      (bind _returnvalue (Game|SpawnActorfromClass "/Game/Blueprints/Max/CameraMode/BP_PhotoModeController.BP_PhotoModeController_C" (Transformation|GetWorldTransform (Variables|Default|GetCamera)) "AdjustIfPossibleButAlwaysSpawn" "MultiplyWithRoot" 0 0))
      (Variables|Default|SetPhotoModeController _returnvalue)
      (Variables|/Game/Blueprints/Max/CameraMode/BP_PhotoModeController.BP_PhotoModeController_C|SetPlayer _returnvalue self)
      (bind _output_get (Variables|/Game/Blueprints/Max/CameraMode/BP_PhotoModeController.BP_PhotoModeController_C|SetPlayerController _returnvalue (Variables|Default|GetPlayerWheelchairController)))
      (Variables|/Game/Blueprints/Radu/Player/WheelchairController/BP_PlayerWheelchairController.BP_PlayerWheelchairController_C|SetControlledPawn (Variables|Default|GetPlayerWheelchairController) _returnvalue)
      (Pawn|Possess _output_get _returnvalue))))

(event Custom|CheckObject
  (params (DeltaSeconds :type Float%20%28single-precision%29))
  (bind _camera (Variables|Default|GetCamera))
  ;[0.15 0.15 0.15 0.5] Object Picked Up Loop
  (if (Variables|Default|GetisGrabbingObject?)
    (Physics|Components|PhysicsHandle|SetTargetLocation (Variables|Default|GetPhysicsHandle) (+ (Transformation|GetWorldLocation _camera) (* (Math|Vector|GetForwardVector (Transformation|GetWorldRotation _camera)) 1e+02)))))

(event Input|EnhancedActionEvents|EnhancedInputActionIA_InteractKeyboard
  (params (ActionValue :type Boolean) (ElapsedSeconds :type Float%20%28double-precision%29) (TriggeredSeconds :type Float%20%28double-precision%29) (InputAction :type Input%20Action%20Object%20Reference :default "/Game/Input/Actions/PlayerWheelchair/Keyboard/IA_InteractKeyboard.IA_InteractKeyboard"))
  (bind _targetdialoguecomponent (Variables|Default|GetTargetDialogueComponent))
  (bind _interactactor (Variables|Default|GetInteractActor))
  (:Started
    (Utilities|FlowControl|Sequence
      (:then_0
        (Utilities|IsValid _targetdialoguecomponent
          (:Is%20Valid
            (Class|BPInteract|Interact(Message) _targetdialoguecomponent self))
          (:Is%20Not%20Valid
            (Development|PrintString "Not Valid Sequence"))))
      (:then_1
        (Utilities|IsValid _interactactor
          (:Is%20Valid
            (Class|BPInteract|Interact(Message) _interactactor self)))))))

(event Input|EnhancedActionEvents|EnhancedInputActionIA_InteractGamepad
  (params (ActionValue :type Boolean) (ElapsedSeconds :type Float%20%28double-precision%29) (TriggeredSeconds :type Float%20%28double-precision%29) (InputAction :type Input%20Action%20Object%20Reference :default "/Game/Input/Actions/PlayerWheelchair/Gamepad/IA_InteractGamepad.IA_InteractGamepad"))
  (bind _targetdialoguecomponent (Variables|Default|GetTargetDialogueComponent))
  (bind _interactactor (Variables|Default|GetInteractActor))
  (:Started
    (Utilities|FlowControl|Sequence
      (:then_0
        (Utilities|IsValid _targetdialoguecomponent
          (:Is%20Valid
            (Class|BPInteract|Interact(Message) _targetdialoguecomponent self))
          (:Is%20Not%20Valid
            (Development|PrintString "Not Valid Sequence"))))
      (:then_1
        (Utilities|IsValid _interactactor
          (:Is%20Valid
            (Class|BPInteract|Interact(Message) _interactactor self)))))))

(event EventBeginPlay
  (bind _returnvalue (Game|GetPlayerCameraManager 0))
  (Components|Activation|SetActive (Variables|Default|GetCamera) true false)
  (Components|Activation|SetActive (Variables|Default|GetCamera1) false false)
  (bind _asbp_player_wheelchair_controller (Utilities|Casting|CastToBP_PlayerWheelchairController (Game|GetPlayerController 0)))
  (Variables|Default|SetPlayerWheelchairController _asbp_player_wheelchair_controller)
  (Variables|/Script/Engine.PlayerCameraManager|SetViewPitchMin _returnvalue -6e+01)
  (Variables|/Script/Engine.PlayerCameraManager|SetViewPitchMax _returnvalue 6e+01)
  (bind _asbp_game_instance (Utilities|Casting|CastToBP_GameInstance (Game|GetGameInstance)))
  (Utilities|FlowControl|Sequence
    (:then_0
      (bind _returnvalue_2 (Game|GetCurrentLevelName true))
      (if (Utilities|Enum|Equal(Enum) _returnvalue_2 "RaduMapGameplay")
        (Default|StartQuest _asbp_game_instance "Enter_Building")))
    (:then_1
      (bind _returnvalue_3 (Game|GetCurrentLevelName true))
      (if (Utilities|Enum|Equal(Enum) _returnvalue_3 "DaniMap")
        (Default|StartQuest _asbp_game_instance "Report_Dryer")
        (Default|StartQuest _asbp_game_instance "Report_Elevator")
        (Default|StartQuest _asbp_game_instance "Report_DoorHandle")))))

(event EventTick
  (params (DeltaSeconds :type Float%20%28single-precision%29))
  (bind _returnvalue (Transformation|GetActorRotation))
  (bind _returnvalue_2 (Game|GetPlayerCameraManager 0))
  (Utilities|FlowControl|Sequence
    (:then_0
      (Variables|/Script/Engine.PlayerCameraManager|SetViewYawMin _returnvalue_2 (- (.yaw _returnvalue) 8e+01))
      (Variables|/Script/Engine.PlayerCameraManager|SetViewYawMax _returnvalue_2 (+ (.yaw _returnvalue) 8e+01)))
    (:then_1
      (CallFunction|CheckObject 0.0))))

(event Input|KeyboardEvents|R
  (params (Key :type Key%20Structure :default "None"))
  (bind _camera (Variables|Default|GetCamera))
  (bind _returnvalue (Transformation|GetWorldLocation _camera))
  ;[0.15 0.04713 0.04713 0.5] Grabbimg System
  (:Pressed
    (bind (_outhit _returnvalue_2) (Collision|LineTraceByChannel _returnvalue (+ _returnvalue (* (Math|Vector|GetForwardVector (Transformation|GetWorldRotation _camera)) 1e+02)) "TraceTypeQuery1" false 0 "None"))
    (if _returnvalue_2
      (Physics|Components|PhysicsHandle|GrabComponentatLocationwithRotation (Variables|Default|GetPhysicsHandle) (.HitComponent (Collision|BreakHitResult _outhit)) "None" (Transformation|GetWorldLocation (.HitComponent (Collision|BreakHitResult _outhit))) "0, 0, 0")
      (Variables|Default|SetisGrabbingObject? true)))
  (:Released
    (if (Variables|Default|GetisGrabbingObject?)
      (Physics|Components|PhysicsHandle|ReleaseComponent (Variables|Default|GetPhysicsHandle)))))

(fn ConstructionScript)