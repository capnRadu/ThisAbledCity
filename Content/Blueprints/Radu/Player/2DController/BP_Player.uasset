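; BP_Player is the player character in the 2DController folder, handling animation triggers and input setup.
; Jump and walk-off-ledge events jump the animation state machine to Airborne, while landing jumps it to Landed and stops movement immediately.
; BeginPlay adds the keyboard camera-mode input mapping context through the player controller.
; A disconnected branch for spawning and possessing a photo mode controller never runs.
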(event EventBeginPlay
  ;[0.15 0.15 0.15 0.5] Adds "IMC_CameraControl" mapping
  (bind _asbp_player_controller (Utilities|Casting|CastToBP_PlayerController (Pawn|GetController)))
  (bind _output_get (Variables|Default|SetAs%20Player%20Controller _asbp_player_controller))
  (Input|AddMappingContext (PlayerController|LocalPlayerSubsystems|GetEnhancedInputLocalPlayerSubsystem _output_get) "/Game/Input/IMCs/Camera/IMC_CameraModeKeyboardControls.IMC_CameraModeKeyboardControls" 0 "(bIgnoreAllPressedKeysUntilRelease=True,bForceImmediately=False,bNotifyUserSettings=False)"))

(event EventOnLanded
  (params (Hit :type Hit%20Result%20Structure%20%28by%20ref%29))
  ;[0.15 0.15 0.15 0.5] Animation triggers
  ;;[0.15 0.15 0.15 0.5] Trigger landing animation
  (Class|PaperZDAnimInstance|JumptoNode (Variables|/Script/PaperZD.PaperZDAnimationComponent|GetAnimInstance (Variables|Default|GetAnimationComponent)) "Landed" "None")
  (Components|Movement|StopMovementImmediately (Variables|Character|GetCharacterMovement)))

(event EventOnJumped
  ;[0.15 0.15 0.15 0.5] Animation triggers
  ;;[0.15 0.15 0.15 0.5] Trigger jumping animation
  (Class|PaperZDAnimInstance|JumptoNode (Variables|/Script/PaperZD.PaperZDAnimationComponent|GetAnimInstance (Variables|Default|GetAnimationComponent)) "Airborne" "None"))

(event EventOnWalkingOffLedge
  (params (PreviousFloorImpactNormal :type Vector%20%28by%20ref%29 :default "0, 0, 0") (PreviousFloorContactNormal :type Vector%20%28by%20ref%29 :default "0, 0, 0") (PreviousLocation :type Vector%20%28by%20ref%29 :default "0, 0, 0") (TimeDelta :type Float%20%28single-precision%29))
  ;[0.15 0.15 0.15 0.5] Animation triggers
  ;;[0.15 0.15 0.15 0.5] Trigger jumping animation
  (Class|PaperZDAnimInstance|JumptoNode (Variables|/Script/PaperZD.PaperZDAnimationComponent|GetAnimInstance (Variables|Default|GetAnimationComponent)) "Airborne" "None"))

(fn ConstructionScript)