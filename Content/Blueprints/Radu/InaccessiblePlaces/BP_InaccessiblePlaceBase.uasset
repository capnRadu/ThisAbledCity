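; Base Blueprint for an inaccessible place in the level that can be recorded as an entry in the player's notebook.
; On its first entry request, it passes its building, room and object names, linked quest and objective IDs, a supplied screenshot and itself to BP_GameInstance.
; A flag prevents duplicate entries.
; A separate event swaps the material on its Cube component.
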(event Custom|SetMaterial
  (params (NewParam :type Material%20Object%20Reference))
  (Rendering|Material|SetMaterial (Variables|Default|GetCube) 0 NewParam))

(event Custom|CreateInaccessiblePlaceEntry
  (params (Screenshot :type Texture%202D%20Object%20Reference))
  (bind _inaccessibleplacedetails (Variables|Default|GetInaccessiblePlaceDetails))
  (if (not (Variables|Default|GetWasEntryCreated))
    (bind _asbp_game_instance (Utilities|Casting|CastToBP_GameInstance (Game|GetGameInstance)))
    (Default|AddNotebookEntry _asbp_game_instance (Utilities|Struct|MakeStruct_InaccessiblePlaceEntry (.buildingname _inaccessibleplacedetails) (.roomname _inaccessibleplacedetails) (.objectname _inaccessibleplacedetails) self Screenshot (.associatedquestid _inaccessibleplacedetails) (.associatedobjectiveid _inaccessibleplacedetails)))
    (Variables|Default|SetWasEntryCreated true)))

(fn ConstructionScript)