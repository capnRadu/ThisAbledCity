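; BP_Objective is a quest objective trigger that completes an objective when the player's wheelchair reaches it.
; Its Sphere overlap accepts only a sphere component tagged InteractCollision on a BP_PlayerWheelchair actor.
; It then passes its QuestID and ObjectiveID to CompleteQuestObjective on BP_GameInstance, with no guard here against repeat overlaps.
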(event OnComponentBeginOverlap(Sphere)
  (params (OverlappedComponent :type Primitive%20Component%20Object%20Reference) (OtherActor :type Actor%20Object%20Reference) (OtherComp :type Primitive%20Component%20Object%20Reference) (OtherBodyIndex :type Integer) (bFromSweep :type Boolean) (SweepResult :type Hit%20Result%20Structure%20%28by%20ref%29))
  (if (and (== (Utilities|GetClass OtherComp) "/Script/Engine.SphereComponent") (Components|ComponentHasTag OtherComp "InteractCollision"))
    (Utilities|Casting|CastToBP_PlayerWheelchair OtherActor)
    (bind _asbp_game_instance (Utilities|Casting|CastToBP_GameInstance (Game|GetGameInstance)))
    (Default|CompleteQuestObjective _asbp_game_instance (Variables|Default|GetQuestID) (Variables|Default|GetObjectiveID))))

(event EventBeginPlay)

(event Collision|EventActorBeginOverlap
  (params (OtherActor :type Actor%20Object%20Reference)))

(event EventTick
  (params (DeltaSeconds :type Float%20%28single-precision%29)))

(fn ConstructionScript)