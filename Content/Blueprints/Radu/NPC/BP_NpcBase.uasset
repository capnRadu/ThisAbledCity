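; BP_NpcBase is a base NPC that starts a quest and turns to face the wheelchair player when they come near.
; Entering the DetectionRadius stores the BP_PlayerWheelchair reference and calls StartQuest on BP_GameInstance with the NPC's QuestID.
; Tick rotates only the actor's yaw toward the stored player, and leaving the radius clears the reference so the turning stops.
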(event OnComponentBeginOverlap(DetectionRadius)
  (params (OverlappedComponent :type Primitive%20Component%20Object%20Reference) (OtherActor :type Actor%20Object%20Reference) (OtherComp :type Primitive%20Component%20Object%20Reference) (OtherBodyIndex :type Integer) (bFromSweep :type Boolean) (SweepResult :type Hit%20Result%20Structure%20%28by%20ref%29))
  (if (!= OtherActor self)
    (bind _asbp_player_wheelchair (Utilities|Casting|CastToBP_PlayerWheelchair OtherActor))
    (Variables|Default|SetPlayer _asbp_player_wheelchair)
    (bind _asbp_game_instance (Utilities|Casting|CastToBP_GameInstance (Game|GetGameInstance)))
    (Default|StartQuest _asbp_game_instance (Variables|Default|GetQuestID))))

(event OnComponentEndOverlap(DetectionRadius)
  (params (OverlappedComponent :type Primitive%20Component%20Object%20Reference) (OtherActor :type Actor%20Object%20Reference) (OtherComp :type Primitive%20Component%20Object%20Reference) (OtherBodyIndex :type Integer))
  (if (!= OtherActor self)
    (Utilities|Casting|CastToBP_PlayerWheelchair OtherActor)
    (Variables|Default|SetPlayer 0)))

(event EventTick
  (params (DeltaSeconds :type Float%20%28single-precision%29))
  (Utilities|IsValid (Variables|Default|GetPlayer)
    (:Is%20Valid
      (Transformation|SetActorRotation self (Math|Rotator|MakeRotator 0.0 0.0 (.yaw (Math|Rotator|FindLookatRotation (Transformation|GetActorLocation) (Transformation|GetActorLocation (Variables|Default|GetPlayer)))))))))

(fn ConstructionScript)